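; Weather actor that runs a repeating rain cycle with random start delay and duration.
; RainTimeline drives storm clouds on a dynamic volumetric cloud material, height fog, and Niagara rain attached to the player pawn, fading looping rain audio at alpha thresholds.
; MaterialTimeline drives "Rain Wetness" in the NPC_Weather parameter collection.
; Its forward finish starts the rain hold, its reversal trails the rain's by a wetness delay, and its reverse finish restarts the cycle.
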(event `self.ReceiveBeginPlay`
  (`|ExecutionSequence`
    (:`then_0`
      (bind _returnvalue (`NiagaraFunctionLibrary.SpawnSystemAttached` "/Game/02_Common/Weather/NS_Rain.NS_Rain" (`Actor.RootComponent` (`Controller.K2_GetPawn` (`GameplayStatics.GetPlayerController` 0))) "None" (0.0 0.0 400.0) (struct) "KeepRelativeOffset"))
      (set `self.Rain Particles` _returnvalue)
      (bind _returnvalue_2 (`KismetMaterialLibrary.CreateDynamicMaterialInstance` (`|ConvertAsset` (`VolumetricCloudComponent.Material` (`self.VolumetricCloud`)))))
      (bind _output_get (set `self.Cloud Material` _returnvalue_2))
      (`VolumetricCloudComponent.SetMaterial` (`self.VolumetricCloud`) _output_get))
    (:`then_1`
      (`self.Init Rain`))))

(event `Init Rain`
  (set `self.Rain Start Delay` (`KismetMathLibrary.RandomFloatInRange` (`self.Rain Start Delay Min`) (`self.Rain Start Delay Max`)))
  (set `self.Rain Duration` (`KismetMathLibrary.RandomFloatInRange` (`self.Rain Duration Min`) (`self.Rain Duration Max`)))
  (`KismetSystemLibrary.K2_SetTimer` null "Begin Rain" (`self.Rain Start Delay`))
  (`KismetSystemLibrary.PrintString` "Init Rain"))

(event `Begin Rain`
  (`KismetSystemLibrary.PrintString` "Begin Rain")
  (`|ExecutionSequence`
    (:`then_0`
      (`TimelineComponent.SetPlayRate` (`self.Material Timeline`) (`self.Trainsition Speed`))
      (`TimelineComponent.SetPlayRate` (`self.Material Timeline`) (`self.Trainsition Speed`)))
    (:`then_1`
      (bind (_direction _rain_effects) (`Timeline|Rain Timeline` :!label _label)
        (:`Update`
          (`MaterialInstanceDynamic.SetScalarParameterValue` (`self.Cloud Material`) "StormClouds" (`KismetMathLibrary.Lerp` 0.02 0.975 _rain_effects))
          (`ExponentialHeightFogComponent.SetFogDensity` (`self.ExponentialHeightFog`) (`KismetMathLibrary.Lerp` 0.02 1.0 _rain_effects))
          (`ExponentialHeightFogComponent.SetFogHeightFalloff` (`self.ExponentialHeightFog`) (`KismetMathLibrary.Lerp` 0.2 1.5 _rain_effects))
          (`NiagaraComponent.SetNiagaraVariableFloat` (`self.Rain Particles`) "Rain Amount" (`KismetMathLibrary.MapRangeClamped` _rain_effects (`self.Rain Min Alpha`) (`self.Rain Max Alpha`) 0.0 1.0))
          (switch `ETimelineDirection` _direction
            (:`Forward`
              (if (>= _rain_effects (`self.Rain Min Alpha`))
                (`/Engine/EditorBlueprintResources/StandardMacros.DoOnce` false :!label _label_2
                  (:`Completed`
                    (`self.Rain Sound`
                      (:`then`
                        _)
                      (:`else`
                        (bind _returnvalue (`GameplayStatics.SpawnSound2D` "/Game/02_Common/Weather/RAINConc_InsJ_Ambience_Rain_Light_01_LOOP_Cue.RAINConc_InsJ_Ambience_Rain_Light_01_LOOP_Cue" 1.0 1.0 0.0 null))
                        (set `self.Rain Sound` _returnvalue)))
                    (`AudioComponent.FadeIn` (`self.Rain Sound`) (/ 2.5 (`self.Trainsition Speed`)) 1.0 0.0 "Linear")))))
            (:`Backward`
              (if (<= _rain_effects (`self.Rain Max Alpha`))
                (`/Engine/EditorBlueprintResources/StandardMacros.DoOnce` false :!label _label_3
                  (:`Completed`
                    (`AudioComponent.FadeOut` (`self.Rain Sound`) (/ 2.5 (`self.Trainsition Speed`)) 0.0 "Linear")))))))))
    (:`then_2`
      (bind (_direction_2 _material_alpha) (`Timeline|Material Timeline` :!label _label_4)
        (:`Update`
          (`KismetMaterialLibrary.SetScalarParameterValue` "/Game/02_Common/Weather/NPC_Weather.NPC_Weather" "Rain Wetness" _material_alpha))
        (:`Finished`
          (switch `ETimelineDirection` _direction_2
            (:`Forward`
              (`KismetSystemLibrary.PrintString` "Rain Full")
              (`KismetSystemLibrary.Delay` (`self.Rain Duration`))
              (`self.End Rain`)
              (`KismetSystemLibrary.PrintString` "Rain End"))
            (:`Backward`
              (`self.Init Rain`)
              (`KismetSystemLibrary.PrintString` "Rain Finished"))))))
    (:`then_3`
      (`self.Reset Do Once Fade Out`))))

(event `End Rain`
  (`|ExecutionSequence`
    (:`then_0`
      (goto _label :!via `Reverse`))
    (:`then_1`
      (`KismetSystemLibrary.Delay` (`self.Material Wetness Duration`))
      (goto _label_4 :!via `Reverse`))
    (:`then_2`
      (`self.Reset Do Once Fade In`))))

(event `Reset Do Once Fade In`
  (goto _label_2 :!via `Reset`))

(event `Reset Do Once Fade Out`
  (goto _label_3 :!via `Reset`))

(fn `UserConstructionScript`)